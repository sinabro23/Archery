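; BP_EnemyDusk is a Minion enemy Blueprint that manages its own health bar widget on top of parent enemy logic.
; On BeginPlay it calls the parent, passes itself to the BP_EnemyHealthBar widget as its Enemy and hides the bar.
; ShowHealthBar and HideHealthBar events toggle the widget's visibility, with only the show event also calling the parent.
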(event EventBeginPlay
  (|CallParentFunction)
  (bind _asbp_enemy_health_bar (Utilities|Casting|CastToBP_EnemyHealthBar (UserInterface|GetUserWidgetObject (Variables|Default|GetHealthBar))))
  (Variables|/Game/_Game/HUD/BP_EnemyHealthBar.BP_EnemyHealthBar_C|SetEnemy _asbp_enemy_health_bar self)
  (Widget|SetVisibility (UserInterface|GetUserWidgetObject (Variables|Default|GetHealthBar)) "Hidden"))

(event EventShowHealthBar
  (Widget|SetVisibility (UserInterface|GetUserWidgetObject (Variables|Default|GetHealthBar)) "Visible")
  (|CallParentFunction))

(event EventHideHealthBar
  (Widget|SetVisibility (UserInterface|GetUserWidgetObject (Variables|Default|GetHealthBar)) "Hidden"))

(fn ConstructionScript)