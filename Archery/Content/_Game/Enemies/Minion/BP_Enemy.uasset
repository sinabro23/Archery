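; BP_Enemy is a minion enemy Blueprint that manages the visibility of its health bar widget.
; On BeginPlay it passes itself to the HealthBar component's BP_EnemyHealthBar widget as its Enemy, then hides the widget.
; ShowHealthBar and HideHealthBar events toggle the widget's visibility, with only the show event also calling its parent implementation.
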(event EventBeginPlay
  (bind _asbp_enemy_health_bar (Utilities|Casting|CastToBP_EnemyHealthBar (UserInterface|GetUserWidgetObject (Variables|Default|GetHealthBar))))
  (Variables|/Game/_Game/HUD/BP_EnemyHealthBar.BP_EnemyHealthBar_C|SetEnemy _asbp_enemy_health_bar self)
  (Widget|SetVisibility (UserInterface|GetUserWidgetObject (Variables|Default|GetHealthBar)) "Hidden"))

(event EventShowHealthBar
  (Widget|SetVisibility (UserInterface|GetUserWidgetObject (Variables|Default|GetHealthBar)) "Visible")
  (|CallParentFunction))

(event EventHideHealthBar
  (Widget|SetVisibility (UserInterface|GetUserWidgetObject (Variables|Default|GetHealthBar)) "Hidden"))

(fn ConstructionScript)