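; BP_RoomGate is a room gate Blueprint with a TextWidget that can be shown or hidden.
; On BeginPlay it casts the component's user widget to GateWidget and stores itself in that widget's GateBP reference, linking the widget back to the gate.
; ShowWidget and HideWidget toggle the user widget's visibility, with no call to either inside this Blueprint.
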(event EventBeginPlay
  (bind _asgate_widget (Utilities|Casting|CastToGateWidget (UserInterface|GetUserWidgetObject (Variables|Default|GetTextWidget))))
  (Variables|/Game/_Game/HUD/GateWidget.GateWidget_C|SetGateBP _asgate_widget self))

(event Collision|EventActorBeginOverlap
  (params (OtherActor :type Actor%20Object%20Reference)))

(event EventTick
  (params (DeltaSeconds :type Float%20%28single-precision%29)))

(event EventShowWidget
  (Widget|SetVisibility (UserInterface|GetUserWidgetObject (Variables|Default|GetTextWidget)) "Visible"))

(event EventHideWidget
  (Widget|SetVisibility (UserInterface|GetUserWidgetObject (Variables|Default|GetTextWidget)) "Hidden"))

(fn ConstructionScript)