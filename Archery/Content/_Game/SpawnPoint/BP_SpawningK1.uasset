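; Spawn point Blueprint that places a mixed group of enemies, made up of Khaimera variants and other enemy types.
; Its EnemySpawn event prints a debug message, spawns each enemy class at its own spawn point, then calls RaiseSpawnCount.
; Nothing in this graph calls EnemySpawn, and the BeginPlay, overlap, Tick and show/hide widget events are empty.
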(event EventBeginPlay)

(event Collision|EventActorBeginOverlap
  (params (OtherActor :type Actor%20Object%20Reference)))

(event EventTick
  (params (DeltaSeconds :type Float%20%28single-precision%29)))

(event EventEnemySpawn
  (Development|PrintText "Hello")
  (Game|SpawnActorfromClass "/Game/_Game/Enemies/Khaimera/BP_Khaimera.BP_Khaimera_C" (Math|Conversions|ToTransform(Vector) (Variables|Default|GetSpawnPoint1)) "Undefined" 0 0)
  (Game|SpawnActorfromClass "/Game/_Game/Enemies/Khaimera/BP_Khaimera1.BP_Khaimera1_C" (Math|Conversions|ToTransform(Vector) (Variables|Default|GetSpawnPoint2)) "Undefined" 0 0)
  (Game|SpawnActorfromClass "/Game/_Game/Enemies/Khaimera/BP_Khaimera2.BP_Khaimera2_C" (Math|Conversions|ToTransform(Vector) (Variables|Default|GetSpawnPoint6)) "Undefined" 0 0)
  (Game|SpawnActorfromClass "/Game/_Game/Enemies/Khaimera/BP_KhaimeraBengal.BP_KhaimeraBengal_C" (Math|Conversions|ToTransform(Vector) (Variables|Default|GetSpawnPoint3)) "Undefined" 0 0)
  (Game|SpawnActorfromClass "/Game/_Game/Enemies/Minion/BP_Enemy.BP_Enemy_C" (Math|Conversions|ToTransform(Vector) (Variables|Default|GetSpawnPoint4)) "Undefined" 0 0)
  (Game|SpawnActorfromClass "/Game/_Game/Enemies/Minion/BP_EnemyDusk.BP_EnemyDusk_C" (Math|Conversions|ToTransform(Vector) (Variables|Default|GetSpawnPoint5)) "Undefined" 0 0)
  (Class|SpawningPoint|RaiseSpawnCount))

(event EventShowWidget)

(event EventHideWidget)

(fn ConstructionScript)